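; Player controller that sets up the inventory and pause menu widgets and handles pausing via the menu button.
; On BeginPlay it creates both widgets, forces a 1080p windowed resolution, starts unpaused in locked game-and-UI input mode, and after a short delay centers the mouse and enables the pawn's tick.
; The menu button, gated by EscEnabled, toggles menu visibility and game pause.
; Any key press shows or hides the cursor depending on gamepad use.
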(event `CustomEvent_0`
  (bind (_returnvalue_x _returnvalue_y) (`KismetMathLibrary.BreakVector2D` (`WidgetLayoutLibrary.GetViewportSize`)))
  (`self.SetMouseLocation` (`KismetMathLibrary.FTrunc` (/ _returnvalue_x 2.0)) (`KismetMathLibrary.FTrunc` (/ _returnvalue_y 2.0)))
  (`self.SetActorTickEnabled` (`GameplayStatics.GetPlayerPawn` 0) true))

(event `Key|AnyKey` :consume false
  (params (Key :type "Key Structure"))
  (:`Pressed`
    (set `self.bShowMouseCursor` (not (`KismetInputLibrary.Key_IsGamepadKey` Key)))))

(event `self.ReceiveBeginPlay`
  (`|ExecutionSequence`
    (:`then_0`
      ;[1 1 1] inventory
      (bind _returnvalue (`|CreateWidget` "/Game/Widgets/pickableUI/WBP_Inventory.WBP_Inventory_C"))
      (bind _output_get (set `self.InventoryWidget` _returnvalue))
      (`UserWidget.AddToViewport` _output_get 0)
      (`KismetSystemLibrary.ExecuteConsoleCommand` "r.setres 1920x1080w" null)
      (`KismetSystemLibrary.K2_SetTimerDelegate` (delegate `CustomEvent_0`) 0.5))
    (:`then_1`
      (bind _returnvalue_2 (`|CreateWidget` "/Game/Widgets/WBP_Menu.WBP_Menu_C" self))
      (bind _output_get_2 (set `self.WBP` _returnvalue_2))
      (`UserWidget.AddToViewport` _output_get_2 0)
      (`self.Unpause`)
      (`WidgetBlueprintLibrary.SetInputMode_GameAndUIEx` self null "LockAlways" false))))

(event `Unpause`
  (set `self.bInMenu` false :!label _label)
  (`Widget.SetVisibility` (`self.WBP`) "Collapsed")
  (`GameplayStatics.SetGamePaused` false))

(event `InputAction|MenuButton` :paused true
  (params (Key :type "Key Structure"))
  (:`Pressed`
    (if (`self.bEscEnabled`)
      (if (`self.bInMenu`)
        (goto _label)
        (else
          (set `self.bInMenu` true)
          (`Widget.SetVisibility` (`self.WBP`) "Visible")
          (`GameplayStatics.SetGamePaused` true))))))

(fn `UserConstructionScript`)