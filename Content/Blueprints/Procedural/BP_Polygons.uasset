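; Actor that builds a tiled grid of regular N-sided polygons, hexagon-style, as a single procedural mesh in the Construction Script.
; Each cell is a triangle fan around a center vertex with radial UVs, offset on odd rows and optionally raised or lowered by random height steps.
; The accumulated arrays get calculated normals, then become one mesh section with the assigned material.
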(event `self.ReceiveTick`
  (params (DeltaSeconds :type "Float (single-precision)")))

(fn `Create Hex`
  (locals (centerX :type "Float (double-precision)") (centerY :type "Float (double-precision)") (centerZ :type "Float (double-precision)"))
  (set `local.centerZ` (`KismetMathLibrary.SelectFloat` (* (+ (`KismetMathLibrary.RandomInteger` 5) -2) 0.5 (`self.Radius`)) 0.0 (`self.bRandomHeight`)))
  (set `local.centerX` (* (+ (* (`self.x`) 2) (mod (`self.y`) 2)) (`self.halfLength`)))
  (set `local.centerY` (* (`self.y`) (`self.Width`)))
  (`KismetArrayLibrary.Array_Add` (`self.Vertices`) (`KismetMathLibrary.MakeVector` (`local.centerX`) (`local.centerY`) (`local.centerZ`))) ; center
  (`KismetArrayLibrary.Array_Add` (`self.UVs`) (0.5 0.5)) ; center
  (for _index (range (`self.AnglesN`))
    (bind _returnvalue (* _index (`self.Degrees`)))
    (bind _returnvalue_2 (`KismetMathLibrary.DegSin` _returnvalue))
    (bind _returnvalue_3 (`KismetMathLibrary.DegCos` _returnvalue))
    (`KismetArrayLibrary.Array_Add` (`self.UVs`) (`KismetMathLibrary.MakeVector2D` (/ (+ _returnvalue_2 1.0) 2.0) (/ (+ _returnvalue_3 1.0) 2.0)))
    (`KismetArrayLibrary.Array_Add` (`self.Vertices`) (`KismetMathLibrary.MakeVector` (+ (* _returnvalue_2 (`self.Radius`)) (`local.centerX`)) (+ (* _returnvalue_3 (`self.Radius`)) (`local.centerY`)) (`local.centerZ`))))
  (`self.MakeTriangles`)
  (return))

(fn `MakeTriangles`
  (locals (HexIndex :type Integer))
  (set `local.HexIndex` (* (+ (* (`self.x`) (`self.Num Y`)) (`self.y`)) (+ (`self.AnglesN`) 1)))
  (for _index (range 2 (+ (`self.AnglesN`) 1))
    ;[0.1927 0.1927 0.1927] 0, 1, 2, 0, 2, 3, 0, 3, 4...
    (`KismetArrayLibrary.Array_Add` (`self.Triangles`) (`local.HexIndex`)) ; 0
    (`KismetArrayLibrary.Array_Add` (`self.Triangles`) (+ (- _index 1) (`local.HexIndex`)))
    (`KismetArrayLibrary.Array_Add` (`self.Triangles`) (+ _index (`local.HexIndex`))))
  ;[0.1927 0.1927 0.1927] 0, last, 1
  (`KismetArrayLibrary.Array_Add` (`self.Triangles`) (`local.HexIndex`))
  (`KismetArrayLibrary.Array_Add` (`self.Triangles`) (+ (`self.AnglesN`) (`local.HexIndex`)))
  (`KismetArrayLibrary.Array_Add` (`self.Triangles`) (+ 1 (`local.HexIndex`))))

(fn `UserConstructionScript`
  (`KismetArrayLibrary.Array_Clear` (`self.Vertices`))
  (`KismetArrayLibrary.Array_Clear` (`self.Triangles`))
  (`KismetArrayLibrary.Array_Clear` (`self.UVs`))
  (set `self.Degrees` (/ 360.0 (`KismetMathLibrary.Conv_IntToDouble` (`self.AnglesN`))))
  (set `self.halfLength` (* (`self.Radius`) (`KismetMathLibrary.DegSin` (* (`self.Degrees`) (`KismetMathLibrary.Conv_IntToDouble` (/ (+ (`self.AnglesN`) 1) 4))))))
  (set `self.Width` (* (`self.Radius`) (+ 1.0 (`KismetMathLibrary.DegCos` (`self.Degrees`)))))
  (for _index (range (`self.Num X`))
    (set `self.x` _index)
    (for _index_2 (range (`self.Num Y`))
      (set `self.y` _index_2)
      (`self.Create Hex`)))
  (bind _normals (`KismetProceduralMeshLibrary.CalculateTangentsForMesh` (`self.Vertices`) (`self.Triangles`) (`self.UVs`)))
  (`ProceduralMeshComponent.CreateMeshSection_LinearColor` :`self` (`self.ProceduralMesh`) :`Vertices` (`self.Vertices`) :`Triangles` (`self.Triangles`) :`Normals` _normals :`UV0` (`self.UVs`))
  (`PrimitiveComponent.SetMaterial` (`self.ProceduralMesh`) 0 (`self.Material`)))