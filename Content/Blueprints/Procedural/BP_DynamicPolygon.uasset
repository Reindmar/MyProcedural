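; Procedural mesh actor that draws a flat regular polygon whose corner count steps up and down between a minimum and maximum over time.
; A looping timer changes the count each cooldown, reversing at the limits, then rebuilds the mesh.
; The rebuild makes a triangle fan from a center vertex with circular UVs, calculated normals and an assigned material.
; The construction script runs the same rebuild.
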(event `self.ReceiveBeginPlay`
  (`KismetSystemLibrary.K2_SetTimerDelegate` (delegate `ChangeAnglesN`) (`self.Cooldown`) true 1.0))

(event `ChangeAnglesN`
  (if (>= (`self.AnglesN`) (`self.MaxAnglesN`))
    (set `self.bIncrease` false)
    (elif (<= (`self.AnglesN`) (`self.MinAnglesN`))
      (set `self.bIncrease` true)))
  (if (`self.bIncrease`)
    (bind _result (`/Engine/EditorBlueprintResources/StandardMacros.IncrementInt` (`self.AnglesN`))
      (:`  `
        (set `self.AnglesN` _result)))
    (else
      (bind _result_2 (`/Engine/EditorBlueprintResources/StandardMacros.DecrementInt` (`self.AnglesN`))
        (:`  `
          (set `self.AnglesN` _result_2)))))
  (`self.Reconsctruct`))

(event `Reconsctruct`
  (`KismetArrayLibrary.Array_Clear` (`self.Vertices`))
  (`KismetArrayLibrary.Array_Clear` (`self.Triangles`))
  (`KismetArrayLibrary.Array_Clear` (`self.UVs`))
  ;[0 0 0 0.411] Creating polygon
  (`KismetArrayLibrary.Array_Add` (`self.Vertices`) (0.0 0.0 0.0)) ; center
  (`KismetArrayLibrary.Array_Add` (`self.UVs`) (0.5 0.5)) ; center
  (for _index (range (`self.AnglesN`))
    (bind _returnvalue (* _index (/ 360.0 (`KismetMathLibrary.Conv_IntToDouble` (`self.AnglesN`)))))
    (bind _returnvalue_2 (`KismetMathLibrary.DegSin` _returnvalue))
    (bind _returnvalue_3 (`KismetMathLibrary.DegCos` _returnvalue))
    (`KismetArrayLibrary.Array_Add` (`self.UVs`) (`KismetMathLibrary.MakeVector2D` (/ (+ _returnvalue_2 1.0) 2.0) (/ (+ _returnvalue_3 1.0) 2.0)))
    (`KismetArrayLibrary.Array_Add` (`self.Vertices`) (`KismetMathLibrary.MakeVector` (* _returnvalue_2 (`self.Radius`)) (* _returnvalue_3 (`self.Radius`)))))
  (for _index_2 (range 2 (+ (`self.AnglesN`) 1))
    ;;[0.1927 0.1927 0.1927] 0, 1, 2, 0, 2, 3, 0, 3, 4...
    (`KismetArrayLibrary.Array_Add` (`self.Triangles`))
    (`KismetArrayLibrary.Array_Add` (`self.Triangles`) (- _index_2 1))
    (`KismetArrayLibrary.Array_Add` (`self.Triangles`) _index_2))
  ;;[0.1927 0.1927 0.1927] 0, last, 1
  (`KismetArrayLibrary.Array_Add` (`self.Triangles`))
  (`KismetArrayLibrary.Array_Add` (`self.Triangles`) (`self.AnglesN`))
  (`KismetArrayLibrary.Array_Add` (`self.Triangles`) 1)
  (bind _normals (`KismetProceduralMeshLibrary.CalculateTangentsForMesh` (`self.Vertices`) (`self.Triangles`) (`self.UVs`)))
  (`ProceduralMeshComponent.CreateMeshSection_LinearColor` :`self` (`self.ProceduralMesh`) :`Vertices` (`self.Vertices`) :`Triangles` (`self.Triangles`) :`Normals` _normals :`UV0` (`self.UVs`))
  (`PrimitiveComponent.SetMaterial` (`self.ProceduralMesh`) 0 (`self.Material`)))

(fn `UserConstructionScript`
  (`self.Reconsctruct`))