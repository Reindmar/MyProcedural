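; Camera pawn that pans, rotates and zooms via keyboard, joystick and mouse.
; Tick prioritizes move input (blended with edge scrolling), then inverted mouse-drag panning, then screen-edge scrolling, with released drags sliding until other movement interrupts.
; Rotation interpolates toward accumulated yaw and clamped pitch, plus a temporary Q/E yaw offset that eases back.
; Zoom interpolates spring arm length on axis input, and ResetCamera restores pitch and the zoom target.
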(event `InputAction|StartMovingCameraWithMouse`
  (params (Key :type "Key Structure"))
  (:`Pressed`
    (set `self.bDragging` true)
    (set `self.DraggingStartPosition` (`self.K2_GetActorLocation`))
    (set `self.DraggingTarget` (0.0 0.0 0.0))
    (set `self.bShouldSlide` true)))

(event `InputAction|StartMovingCameraWithMouse` :paused true
  (params (Key :type "Key Structure"))
  (:`Released`
    (set `self.bDragging` false)))

(event `self.ReceiveTick`
  (params (DeltaSeconds :type "Float (single-precision)"))
  (bind (_returnvalue_x _returnvalue_y) (`KismetMathLibrary.BreakVector` (`self.GetActorForwardVector`)))
  (bind (_returnvalue_x_2 _returnvalue_y_2) (`KismetMathLibrary.BreakVector` (`self.GetActorRightVector`)))
  (bind _returnvalue (`GameplayStatics.GetWorldDeltaSeconds`))
  (bind _returnvalue_2 (`KismetMathLibrary.FMax` (`self.NextMoveStrength`) (`self.BorderStrength`)))
  (bind _returnvalue_3 (* _returnvalue_2 -1.0))
  (`|ExecutionSequence`
    (:`then_0`
      (if (or (!= (`self.GetInputAxisValue`) 0.0) (!= (`self.GetInputAxisValue`) 0.0)) :!pinned true
        (`self.Set Up BorderAxis`) ; WASD/Joystick=1
        (set `self.bShouldSlide` false :!label _label)
        ;[0.001789 0.008759 0.009375] Camera Movement
        (`self.AddMovementInput` (`KismetMathLibrary.MakeVector` _returnvalue_x _returnvalue_y) (* (`KismetMathLibrary.FClamp` (+ (* (`self.GetInputAxisValue`) (`self.NextMoveStrength`)) (* (`self.BorderAxisX`) (`self.BorderStrength`))) _returnvalue_3 _returnvalue_2) _returnvalue)) ; z=0
        (`self.AddMovementInput` (`KismetMathLibrary.MakeVector` _returnvalue_x_2 _returnvalue_y_2) (* _returnvalue (`KismetMathLibrary.FClamp` (+ (* (`self.GetInputAxisValue`) (`self.NextMoveStrength`)) (* (`self.BorderAxisY`) (`self.BorderStrength`))) _returnvalue_3 _returnvalue_2))) ; z=0
        (else
          (if (`self.bDragging`) :!pinned true
            (set `self.DraggingTarget` (- (`self.DraggingTarget`) (`KismetMathLibrary.TransformDirection` (`KismetMathLibrary.MakeTransform` (0.0 0.0 0.0) (`KismetMathLibrary.MakeRotator` 0.0 0.0 (.yaw (.rotation (`self.GetTransform`))))) (`KismetMathLibrary.MakeVector` (`self.GetInputAxisValue`) (`self.GetInputAxisValue`))))) ; WASD/Joystick=0, Dragging=1
            (else
              (`self.Set Up BorderAxis`) ; WASD/Joystick=0, Dragging=0
              (if (`self.CursorNearBorder`) :!pinned true
                (goto _label)
                (else
                  _))))
          (if (`self.bShouldSlide`) :!pinned true
            ;[0.01771 0 0.000799] on LMB Slide
            (`self.K2_SetActorLocation` (`KismetMathLibrary.VInterpTo` (`self.K2_GetActorLocation`) (+ (`self.DraggingStartPosition`) (* (`self.DraggingTarget`) (`self.DraggingStrength`))) (`GameplayStatics.GetWorldDeltaSeconds`) (`self.SlideInterpSpeed`)))))))
    (:`then_1`
      ;[0.001789 0.008759 0.009375] Camera Rotation
      (if (`self.bRotating`)
        (`self.Update RotatingTarget` (`self.GetInputAxisValue`) (`self.GetInputAxisValue`))
        (else
          (`self.Update RotatingTarget` 0.0)))
      (if (not (== (`self.GetInputAxisValue`) 0.0))
        (set `self.bResetRotation` false))
      (`self.Update RotationZ`)
      (`self.K2_SetActorRotation` (`KismetMathLibrary.RInterpTo` (`self.K2_GetActorRotation`) (`KismetMathLibrary.MakeRotator` 0.0 (`self.RotatingTargetY`) (+ (`self.RotatingTargetX`) (`self.RotationZ`))) (`GameplayStatics.GetWorldDeltaSeconds`) (`self.RotatingInterpSpeed`))))))

(event `InputAction|StartRotatingCameraWithMouse`
  (params (Key :type "Key Structure"))
  ;[0.001789 0.008759 0.009375] Camera Rotation
  (:`Pressed`
    (set `self.bRotating` true)
    (set `self.bResetRotation` false)))

(event `InputAction|StartRotatingCameraWithMouse` :paused true
  (params (Key :type "Key Structure"))
  ;[0.001789 0.008759 0.009375] Camera Rotation
  (:`Released`
    (set `self.bRotating` false)))

(event `InputAction|ResetCamera`
  (params (Key :type "Key Structure"))
  (:`Pressed`
    (`|ExecutionSequence`
      (:`then_0`
        ;[0.001789 0.008759 0.009375] Camera Rotation
        (set `self.bResetRotation` true))
      (:`then_1`
        ;[0 0 0 0.333] Zoom
        (set `self.ZoomingTarget` 700.0)))))

(event `InputAxis|CameraZoom`
  (params (AxisValue :type "Float (single-precision)"))
  ;[0 0 0 0.333] Zoom
  (bind _output_get (set `self.ZoomingTarget` (`KismetMathLibrary.FClamp` (+ (`self.ZoomingTarget`) (* AxisValue (`self.ZoomingStrength`))) (`self.ZoomingMinDistance`) (`self.ZoomingMaxDistance`))))
  (set `SpringArmComponent.TargetArmLength` (`KismetMathLibrary.FInterpTo` (`SpringArmComponent.TargetArmLength` (`self.SpringArm`)) _output_get (`GameplayStatics.GetWorldDeltaSeconds`) (`self.ZoomingInterpSpeed`)) (`self.SpringArm`)))

(fn `Set Up BorderAxis`
  (bind _bordersize (`self.BorderSize`))
  (set `self.CursorNearBorder` false)
  (set `self.BorderAxisY` 0.0)
  (set `self.BorderAxisX` 0.0)
  (if (not (`self.bRotating`))
    (bind _returnvalue (`WidgetLayoutLibrary.GetMousePositionOnViewport`))
    (bind _returnvalue_2 (`WidgetLayoutLibrary.GetViewportWidgetGeometry`))
    (`|ExecutionSequence`
      (:`then_0`
        (if (<= (`KismetMathLibrary.BreakVector2D` _returnvalue) (`self.BorderSize`))
          (set `self.BorderAxisY` -1.0)
          (set `self.CursorNearBorder` true :!label _label)
          (else
            (bind (_returnvalue_x _returnvalue_y) (`KismetMathLibrary.BreakVector2D` (`SlateBlueprintLibrary.GetLocalSize` _returnvalue_2)))
            (if (>= (`KismetMathLibrary.BreakVector2D` _returnvalue) (- _returnvalue_x _bordersize))
              (set `self.BorderAxisY` 1.0)
              (goto _label)))))
      (:`then_1`
        (if (>= (`.Y` (`KismetMathLibrary.BreakVector2D` _returnvalue)) (- _returnvalue_y _bordersize))
          (set `self.BorderAxisX` -1.0)
          (goto _label)
          (elif (<= (`.Y` (`KismetMathLibrary.BreakVector2D` _returnvalue)) (`self.BorderSize`))
            (set `self.BorderAxisX` 1.0)
            (goto _label)))))))

(fn `Update RotatingTarget`
  (params (InputX :type "Float (double-precision)") (InputY :type "Float (double-precision)"))
  (set `self.RotatingTargetX` (+ InputX (`self.RotatingTargetX`) (`self.GetInputAxisValue`)))
  (set `self.RotatingTargetY` (`KismetMathLibrary.SelectFloat` (`KismetMathLibrary.FInterpTo` (`self.RotatingTargetY`) 0.0 (`GameplayStatics.GetWorldDeltaSeconds`) (`self.ResetCameraInterpSpeed`)) (`KismetMathLibrary.FClamp` (+ InputY (`self.RotatingTargetY`) (`self.GetInputAxisValue`)) -20.0 65.0) (`self.bResetRotation`))))

(fn `Update RotationZ`
  (set `self.RotationZ` (`KismetMathLibrary.FInterpTo` (`self.RotationZ`) (* (`KismetMathLibrary.FClamp` (`self.GetInputAxisValue`) -1.0) (`self.MaxAngleZ`)) (`GameplayStatics.GetWorldDeltaSeconds`) (`self.RotationZInterpSpeed`))))

(fn `UserConstructionScript`)