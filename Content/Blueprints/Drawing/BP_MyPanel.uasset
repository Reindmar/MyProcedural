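; Paintable panel that lets the player draw and erase on a render target with mouse or joystick input.
; Each tick it traces the panel mesh from the cursor or camera forward, shows a debug sphere, and feeds the hit UV to a dynamic brush material.
; Drawing writes directly to the painting target, while erasing, which takes priority, accumulates in a separate target that is subtracted from the painting on button release.
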(event `self.ReceiveBeginPlay`
  (bind _rt_painting (`self.RT_Painting`))
  (`KismetRenderingLibrary.ClearRenderTarget2D` _rt_painting (`TextureRenderTarget2D.ClearColor` _rt_painting))
  (bind _returnvalue (`KismetMaterialLibrary.CreateDynamicMaterialInstance` (`self.PaintingBrush`)))
  (bind _output_get (set `self.PaintingBrush Instance` _returnvalue))
  (`MaterialInstanceDynamic.SetScalarParameterValue` _output_get "BrushSize" (`self.BrushSize`))
  (`MaterialInstanceDynamic.SetScalarParameterValue` _output_get "BrushHardness" (`self.BrushHardness`)))

(event `InputAction|DrawToCanvas`
  (params (Key :type "Key Structure"))
  (bind _rt_deleting (`self.RT_Deleting`))
  ;[0 0 0 1 14] If both buttons are pressed, it will draw and delete at the same time -> same outcome as if only using delete button
  (:`Pressed`
    (set `self.bMouse` true)
    (set `self.Draw` true :!label _label))
  (:`Released`
    (set `self.Draw` false :!label _label_2)
    (set `self.Delete` false)
    (if (`self.bShouldClear`)
      (`KismetRenderingLibrary.DrawMaterialToRenderTarget` (`self.RT_Painting`) (`self.SubstractionBrush`) :!pinned true) ; Substract RT_Deleting from RT_Painting
      (`KismetRenderingLibrary.ClearRenderTarget2D` _rt_deleting (`TextureRenderTarget2D.ClearColor` _rt_deleting)) ; Clear RT_Deleting
      (set `self.bShouldClear` false))))

(event `InputAction|DeleteFromCanvas`
  (params (Key :type "Key Structure"))
  ;[0 0 0 1 14] If both buttons are pressed, it will draw and delete at the same time -> same outcome as if only using delete button
  (:`Pressed`
    (set `self.bMouse` true)
    (set `self.Delete` true :!label _label_3))
  (:`Released`
    (goto _label_2)))

(event `self.ReceiveTick`
  (params (DeltaSeconds :type "Float (single-precision)"))
  (bind _paintingbrush_instance (`self.PaintingBrush Instance`))
  (bind _uv (`GameplayStatics.FindCollisionUV` (`self.Hit`)))
  (bind _transformcomponent (`PlayerCameraManager.TransformComponent` (`GameplayStatics.GetPlayerCameraManager` 0)))
  (bind _returnvalue (`SceneComponent.K2_GetComponentLocation` _transformcomponent))
  (bind (_bblockinghit _binitialoverlap _time _distance _location _impactpoint _normal _impactnormal _physmat _hitactor _hitcomponent _hitbonename _bonename _hititem _elementindex _faceindex _tracestart _traceend) (`GameplayStatics.BreakHitResult` (`PlayerController.GetHitResultUnderCursorByChannel` (`GameplayStatics.GetPlayerController` 0) "TraceTypeQuery1" true)))
  (if (`self.bMouse`)
    (bind (_hitlocation _hitnormal _bonename_2 _outhit _returnvalue_2) (`PrimitiveComponent.K2_LineTraceComponent` (`self.PanelMesh`) _tracestart _traceend true false false))
    (if _returnvalue_2
      (set `self.Hit` _outhit)
      (`KismetSystemLibrary.DrawDebugSphere` (`.Location` (`GameplayStatics.BreakHitResult` (`self.Hit`))) 10.0 12 (`KismetMathLibrary.SelectColor` (struct :`R` 0.989934 :`G` 1.0 :`A` 1.0) (struct :`R` 1.0 :`G` 1.0 :`B` 1.0 :`A` 1.0) (or (`self.Draw`) (`self.Delete`))) 0.0625 1.0 :!label _label_4)
      (if (`self.Delete`)
        (`MaterialInstanceDynamic.SetVectorParameterValue` _paintingbrush_instance "BrushPosition" (make `LinearColor` (`KismetMathLibrary.BreakVector2D` _uv) (`.Y` (`KismetMathLibrary.BreakVector2D` _uv)) 1.0 1.0)) ; 1 in Blue
        (`KismetRenderingLibrary.DrawMaterialToRenderTarget` (`self.RT_Deleting`) _paintingbrush_instance) ; Draw to RT_Deleting what to delete from RT_Painting
        (set `self.bShouldClear` true)
        (elif (`self.Draw`)
          (`MaterialInstanceDynamic.SetVectorParameterValue` _paintingbrush_instance "BrushPosition" (make `LinearColor` (`KismetMathLibrary.BreakVector2D` _uv) (`.Y` (`KismetMathLibrary.BreakVector2D` _uv)) 0.0 1.0)) ; 0 in Blue
          (`KismetRenderingLibrary.DrawMaterialToRenderTarget` (`self.RT_Painting`) _paintingbrush_instance) ; Draw to RT_Painting
        )))
    (else
      (bind (_hitlocation_2 _hitnormal_2 _bonename_3 _outhit_2 _returnvalue_3) (`PrimitiveComponent.K2_LineTraceComponent` (`self.PanelMesh`) _returnvalue (+ _returnvalue (* (`SceneComponent.GetForwardVector` _transformcomponent) (`self.RayLength`))) true false false))
      (if _returnvalue_3
        (set `self.Hit` _outhit_2)
        (goto _label_4)))))

(event `InputAction|DrawToCanvasJoystick`
  (params (Key :type "Key Structure"))
  ;[0 0 0 1 14] If both buttons are pressed, it will draw and delete at the same time -> same outcome as if only using delete button
  (:`Pressed`
    (set `self.bMouse` false)
    (goto _label))
  (:`Released`
    (goto _label_2)))

(event `InputAction|DeleteFromCanvasJoystick`
  (params (Key :type "Key Structure"))
  ;[0 0 0 1 14] If both buttons are pressed, it will draw and delete at the same time -> same outcome as if only using delete button
  (:`Pressed`
    (set `self.bMouse` false)
    (goto _label_3))
  (:`Released`
    (goto _label_2)))

(fn `UserConstructionScript`)